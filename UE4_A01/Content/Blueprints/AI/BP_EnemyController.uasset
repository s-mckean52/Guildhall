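; BP_EnemyController is the AI controller for enemy characters, linking perception to their behavior tree.
; On possession it runs BT_EnemyCharacter.
; When AI perception successfully senses an actor tagged Player, it sets the line-of-sight flag and stores that actor in the Blackboard.
; Failed sensing updates are ignored, so this controller never clears either key.
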(event `self.ReceivePossess`
  (params (PossessedPawn :type "Pawn Object Reference"))
  (`self.RunBehaviorTree` "/Game/Blueprints/AI/BT_EnemyCharacter.BT_EnemyCharacter"))

(event `self.AIPerception.OnTargetPerceptionUpdated`
  (params (Actor :type "Actor Object Reference") (Stimulus :type "AIStimulus Structure"))
  (bind _blackboard (`self.Blackboard`))
  (if (and (`self.ActorHasTag` Actor "Player") (`.bSuccessfullySensed` (break `AIStimulus` Stimulus)))
    (`BlackboardComponent.SetValueAsBool` _blackboard (`self.HasLineOfSightName`) true)
    (`BlackboardComponent.SetValueAsObject` _blackboard (`self.EnemyActorName`) Actor)))

(fn `UserConstructionScript`)